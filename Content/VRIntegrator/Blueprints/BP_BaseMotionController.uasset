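; Base VR motion controller actor that holds hand setup and thumbstick state for a VR pawn.
; SetupControllerMesh sets the motion source from the Hand enum and scales the mesh by the pawn's world scale, mirroring Y for Oculus right hands.
; It also flags the HMD type and lowers haptic strength on SteamVR.
; Empty trigger, grip and post-creation functions act as hooks, presumably for child controllers.
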(event EventBeginPlay
  (|CallParentFunction))

(event Collision|EventActorBeginOverlap
  (params (OtherActor :type Actor%20Object%20Reference)))

(event EventTick
  (params (DeltaSeconds :type Float%20%28single-precision%29)))

(fn ConstructionScript)

(fn SetThumbstickRotation
  (params (InRotation :type Rotator) (InRotationNoOffset :type Rotator) (InUpAxis :type Float%20%28single-precision%29) (InRightAxis :type Float%20%28single-precision%29))
  (Variables|Default|SetThumbstickRotation InRotation)
  (Variables|Default|SetThumbstickRotationNoOffset InRotationNoOffset)
  (Variables|Default|SetThumbstickUpAxis InUpAxis)
  (Variables|Default|SetThumbstickRightAxis InRightAxis))

(fn SetupControllerMesh
  (params (InMeshComponent :type Scene%20Component%20Object%20Reference))
  (LocalVariables|SetMeshComponent InMeshComponent)
  (bind _out_scalefactor (Default|GetWorldScaleFactor (Variables|Default|GetParentVRBasePawn)))
  (LocalVariables|SetMeshScale (Math|Vector|MakeVector _out_scalefactor _out_scalefactor _out_scalefactor))
  (Variables|/Script/HeadMountedDisplay.MotionControllerComponent|SetMotionSource (Variables|Default|GetMotionController) (Utilities|Name|EnumtoName (Variables|Default|GetHand)))
  (Utilities|FlowControl|Sequence
    (:then_0
      (switch name (Class|HeadMountedDisplayFunctionLibrary|GetHMDDeviceName)
        (:OculusHMD
          (Variables|Default|SetIsOculusHMD true))
        (:SteamVR
          (Variables|Default|SetIsSteamVR true)
          (Variables|Default|SetHapticMultiplier 0.3))
        (:PSVR
          (Variables|Default|SetIsPSVR true))))
    (:then_1
      (switch Utilities|FlowControl|Switch|SwitchonEControllerHand (Variables|Default|GetHand)
        (:Right
          (if (Variables|Default|GetIsOculusHMD)
            (LocalVariables|SetMeshScale (* (LocalVariables|GetMeshScale) "1.000000,-1.000000,1.000000"))))))
    (:then_2
      (Transformation|SetRelativeScale3D (LocalVariables|GetMeshComponent) (LocalVariables|GetMeshScale)))))

(fn InputTriggerPressed)

(fn InputTriggerReleased)

(fn InputGrip1Pressed)

(fn InputGrip1Released)

(fn OnPostCreation)