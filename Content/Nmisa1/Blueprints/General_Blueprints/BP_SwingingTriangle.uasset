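; BP_SwingingTriangle is an actor that swings a triangle through custom events.
; RotateTrianglePivot randomizes a timeline length, then plays a timeline that sets actor rotation and spawns a BP_NumberPad at a fixed transform on every update.
; Separately, ReturnRotate re-arms itself by timer, issuing opposing eased MoveComponentTo tilts on the root, directly and through StartRotate.
; Once game time passes StopTime, it also calls StopRotate to halt the component move.
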(event Custom|StartRotate
  (Components|MoveComponentTo (Variables|Default|GetDefaultSceneRoot) (Variables|Default|GetConstantPosition) "2.000000, 0, 0" true true 1.0 false))

(event Custom|ReturnRotate
  (params (RotateTriangle :type Actor%20Object%20Reference))
  (Components|MoveComponentTo (Variables|Default|GetDefaultSceneRoot) (Variables|Default|GetConstantPosition) "-2.000000, 0, 0" true true 1.0 false)
  (CallFunction|StartRotate)
  (Utilities|Time|SetTimerbyFunctionName "BP_SwingingTriangle" "ReturnRotate" 1.0)
  (if (> (Utilities|Time|GetGameTimeinSeconds) (Variables|Default|GetStopTime))
    (CallFunction|StopRotate)))

(event Custom|StopRotate
  (params (StopTriangle :type BP%20Swinging%20Triangle%20Object%20Reference))
  (Components|MoveComponentTo (Variables|Default|GetDefaultSceneRoot) (Variables|Default|GetConstantPosition) "0, 0, 0" true true 1.0 false) ; enters at Stop
)

(event Custom|RotateTrianglePivot
  (params (RotateTriangle :type BP%20Swinging%20Triangle%20Object%20Reference))
  ;[1 1 1] Swing Triangle
  (Components|Timeline|SetTimelineLength (Variables|Default|GetSwinging_Triangle) (Math|Random|RandomFloatinRange 1.0 12.0))
  (bind _rotatetriangle (Timeline|Swinging_Triangle Play)
    (:Update
      (Transformation|SetActorRotation (Math|Rotator|MakeRotator (.x _rotatetriangle) (.y _rotatetriangle) (.z _rotatetriangle)))
      (Game|SpawnActorfromClass "/Game/Nmisa1/Blueprints/Calibration_BPs/NumberPad/BP_NumberPad.BP_NumberPad_C" (Math|Transform|MakeTransform "-365.000000,406.000000,126.000000" "0, 0, 0" "0.400000,0.400000,0.400000") "Undefined" 0 0))))

(event EventBeginPlay)

(event Collision|EventActorBeginOverlap
  (params (OtherActor :type Actor%20Object%20Reference)))

(event EventTick
  (params (DeltaSeconds :type Float%20%28single-precision%29)))

(fn ConstructionScript)