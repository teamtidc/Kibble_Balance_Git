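; Laser emitter actor for a mirror puzzle that repeatedly casts a light ray along the LaserEmitter's up vector from delayed Tick.
; CastLight loops line traces, bouncing off hit faces with the Mirror material via offset-adjusted normal reflection, and stops otherwise.
; Each bounce calls LaserHitsMirror on all Watt_Balance_Light_Blueprint actors.
; The ray shows only as debug trace lines, since the beam-particle setters are unconnected.
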(event EventTick
  (params (DeltaSeconds :type Float%20%28single-precision%29))
  (bind _laseremitter (Variables|Default|GetLaserEmitter))
  (bind _returnvalue (Transformation|GetWorldLocation _laseremitter))
  (Utilities|FlowControl|Delay 0.01)
  (CallFunction|CastLight _returnvalue (+ _returnvalue (* (Math|Vector|GetUpVector _laseremitter) 3e+04)) (Variables|Default|GetCastDistance)))

(fn ConstructionScript)

(fn CastLight
  (params (CastOrigin :type Vector) (CastDirection :type Vector) (CastDistance :type Float%20%28single-precision%29))
  ;[1 1 1] Create Light Beam
  (LocalVariables|SetL_CastOrigin CastOrigin)
  (LocalVariables|SetL_CastDirection CastDirection)
  (LocalVariables|SetL_CastDistance CastDistance)
  (while (LocalVariables|GetL_Continue)
    (bind (_outhit _returnvalue) (Collision|LineTraceByChannel (LocalVariables|GetL_CastOrigin) (+ (LocalVariables|GetL_CastOrigin) (+ (LocalVariables|GetL_CastDirection) (LocalVariables|GetL_CastDistance))) "TraceTypeQuery3" true 0 "ForDuration" true "(R=1.000000,G=0.000000,B=0.000000,A=1.000000)" "(R=0.021329,G=0.432292,B=0.053760,A=1.000000)"))
    (if _returnvalue
      (if (== (.ReturnValue (Class|PrimitiveComponent|GetMaterialfromCollisionFaceIndex (.HitComponent (Collision|BreakHitResult _outhit)) (.FaceIndex (Collision|BreakHitResult _outhit)))) "/Game/Nmisa1/Assets/Textures_And_Materials/Materials/Mirror.Mirror")
        (LocalVariables|SetL_CastOrigin (.ImpactPoint (Collision|BreakHitResult _outhit)))
        (LocalVariables|SetL_CastDirection (Math|Vector|MirrorVectorbyNormal (- (LocalVariables|GetL_CastDirection) 5e+02) (Math|Vector|MakeVector (+ (.x (.ImpactNormal (Collision|BreakHitResult _outhit))) 1.613) (+ (.y (.ImpactNormal (Collision|BreakHitResult _outhit))) 0.0) (+ (.z (.ImpactNormal (Collision|BreakHitResult _outhit))) 1.79))))
        (bind _outactors (Actor|GetAllActorsOfClass "/Game/Nmisa1/Blueprints/Watt_Balance_Light_Blueprint.Watt_Balance_Light_Blueprint_C"))
        (Default|LaserHitsMirror _outactors)
        (LocalVariables|SetL_Continue true)
        (else
          (LocalVariables|SetL_Continue false :!label _label)))
      (else
        (goto _label)))))