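; BP_Knob is a hand-driven lever that starts or stops a rotating triangle.
; OnDrag converts the current interactor's position to actor space, takes its Atan2 angle and applies it as clamped pitch to LeverRotate.
; Release calls RotateTrianglePivot at maximum pitch and StopRotate at minimum.
; Grab attaches the Knob to the given component and sets its world rotation, while CanBeGrabbed always returns false.
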(event EventBeginPlay
  (Variables|Default|SetInitialLeverRotation (Variables|/Script/Engine.SceneComponent|GetRelativeRotation (Variables|Default|GetLeverRotate))))

(event Collision|EventActorBeginOverlap
  (params (OtherActor :type Actor%20Object%20Reference)))

(event EventTick
  (params (DeltaSeconds :type Float%20%28single-precision%29)))

(event EventGrab
  (params (AttachTo :type Scene%20Component%20Object%20Reference) (SocketName :type Name :default "None") (Hand :type EControllerHand%20Enum :default "Left"))
  (bind _returnvalue (Transformation|AttachComponentToComponent (Variables|Default|GetKnob) AttachTo SocketName "KeepWorld" "KeepWorld" "KeepWorld" true))
  (bind _output_get (Variables|Default|SetIsReadyToRotate _returnvalue))
  (if _output_get
    (Transformation|SetWorldRotation (Variables|Default|GetKnob) "180.000000,-180.000000, 0" false false)
    (else
      (Transformation|SetWorldRotation (Variables|Default|GetKnob) "0,-180.000000, 0" false false))))

(event EventRelease
  (if (== (Variables|Default|GetCurrentPitch) (Variables|Default|GetMaxPitch))
    (Default|RotateTrianglePivot (Variables|Default|GetRotateTriangle))
    (elif (== (Variables|Default|GetCurrentPitch) (Variables|Default|GetMinPitch))
      (Default|StopRotate (Variables|Default|GetStopTriangle)))))

(fn ConstructionScript)

(fn CanbeGrabbed
  (return false))

(fn OnDrag
  (params (Iterator :type Scene%20Component%20Object%20Reference))
  (bind _returnvalue (Transformation|GetActorTransform))
  (bind _currentinteractor (Variables|Default|GetCurrentInteractor))
  (bind _returnvalue_2 (Transformation|GetWorldLocation _currentinteractor))
  (bind _returnvalue_3 (Math|Transform|InverseTransformLocation _returnvalue _returnvalue_2))
  (bind _returnvalue_4 (Math|Vector|UnrotateVector _returnvalue_3 "90.000000, 0, 0"))
  ;[1 1 1] Rotate Knob
  (if (== Iterator (Variables|Default|GetCurrentInteractor))
    (if (not (Variables|Default|GetIsResettingRotation))
      (bind _output_get (Variables|Default|SetCurrentPitch (Math|Float|Clamp(Float) (Class|KismetMathLibrary|DegAtan2 (.z _returnvalue_4) (.x _returnvalue_4)) (Variables|Default|GetMinPitch) (Variables|Default|GetMaxPitch))))
      (Transformation|SetRelativeRotation (Variables|Default|GetLeverRotate) (Math|Rotator|MakeRotator 0.0 _output_get 0.0) false false))
    (else
      (return false))))