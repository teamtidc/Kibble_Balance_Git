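; BP_Identify_Scales is an interactable, non-grabbable scales actor with a world-space popup widget, used with VR pointer motion controllers.
; While the popup is visible, Tick turns it on yaw only to face the player camera.
; On trigger press, it reads the first pointer controller's last laser hit and shows that actor if it is a BP_DockableWindow.
; Trigger box events are empty, and the Scale_Popup show and hide logic is disconnected.
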(event OnComponentBeginOverlap(TriggerBox)
  (params (OverlappedComponent :type Primitive%20Component%20Object%20Reference) (OtherActor :type Actor%20Object%20Reference) (OtherComp :type Primitive%20Component%20Object%20Reference) (OtherBodyIndex :type Integer) (bFromSweep :type Boolean) (SweepResult :type Hit%20Result%20Structure%20%28by%20ref%29)))

(event OnComponentEndOverlap(TriggerBox)
  (params (OverlappedComponent :type Primitive%20Component%20Object%20Reference) (OtherActor :type Actor%20Object%20Reference) (OtherComp :type Primitive%20Component%20Object%20Reference) (OtherBodyIndex :type Integer)))

(event OnComponentHit(TriggerBox)
  (params (HitComponent :type Primitive%20Component%20Object%20Reference) (OtherActor :type Actor%20Object%20Reference) (OtherComp :type Primitive%20Component%20Object%20Reference) (NormalImpulse :type Vector :default "0, 0, 0") (Hit :type Hit%20Result%20Structure%20%28by%20ref%29)))

(event EventBeginPlay)

(event Collision|EventActorBeginOverlap
  (params (OtherActor :type Actor%20Object%20Reference)))

(event EventTick
  (params (DeltaSeconds :type Float%20%28single-precision%29))
  (if (Variables|/Script/Engine.SceneComponent|GetbVisible (Variables|Default|GetPopupUI))
    (CallFunction|UpdatePopupFacing)))

(event EventTriggerPressed
  (bind _outactors (Actor|GetAllActorsOfClass "/Game/VRIntegrator/Blueprints/BP_PointerMotionController.BP_PointerMotionController_C"))
  (bind _asbp_pointer_motion_controller (Utilities|Casting|CastToBP_PointerMotionController (Utilities|Array|Get(acopy) _outactors)))
  (Variables|/Game/VRIntegrator/Blueprints/BP_PointerMotionController.BP_PointerMotionController_C|SetLastLaserHitResult _asbp_pointer_motion_controller (Variables|/Game/VRIntegrator/Blueprints/BP_PointerMotionController.BP_PointerMotionController_C|GetLastLaserHitResult _asbp_pointer_motion_controller))
  (bind _asbp_dockable_window (Utilities|Casting|CastToBP_DockableWindow (.HitActor (Collision|BreakHitResult (Variables|/Game/VRIntegrator/Blueprints/BP_PointerMotionController.BP_PointerMotionController_C|GetLastLaserHitResult _asbp_pointer_motion_controller)))))
  (Default|ShowDockableWindow _asbp_dockable_window true false))

(event EventTriggerReleased)

(fn ConstructionScript)

(fn UpdatePopupFacing
  (Transformation|SetWorldRotation (Variables|Default|GetPopupUI) (Math|Rotator|MakeRotator 0.0 0.0 (.yaw (Math|Rotator|FindLookatRotation (Transformation|GetWorldLocation (Variables|Default|GetPopupUI)) (Camera|GetCameraLocation (Game|GetPlayerCameraManager 0))))) false false))

(fn CanbeGrabbed
  (return false))

(fn OnDrag
  (params (Iterator :type Scene%20Component%20Object%20Reference))
  (return false))